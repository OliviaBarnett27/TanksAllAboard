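; BP_SlidingDoor is a two-panel sliding door that opens when something begins overlapping its box collision.
; BeginPlay caches both panels' world locations, then two timelines drive lerps that slide them 200 units apart along world Y, regardless of actor rotation.
; The right timeline's Update plays the left timeline, whose Update moves both panels.
; The overlapping actor is not filtered, and no logic closes the door.
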(event `self.Box Collision.OnComponentBeginOverlap`
  (params (OverlappedComponent :type "PrimitiveComponent Object Reference") (OtherActor :type "Actor Object Reference") (OtherComp :type "PrimitiveComponent Object Reference") (OtherBodyIndex :type Integer) (bFromSweep :type Boolean) (SweepResult :type "HitResult Structure (by ref)"))
  (bind _rightstartlocation (`self.RightStartLocation`))
  (bind _leftstartlocation (`self.LeftStartLocation`))
  (bind (_direction _alpha) (`Timeline|TL_RightMovement`)
    (:`Update`
      (bind (_direction_2 _alpha_2) (`Timeline|TL_LeftMovement`)
        (:`Update`
          (`SceneComponent.K2_SetWorldLocation` (`self.LeftDoor`) (`KismetMathLibrary.VLerp` _leftstartlocation (+ _leftstartlocation (0.0 200.0 0.0)) _alpha_2) false false)
          (`SceneComponent.K2_SetWorldLocation` (`self.RightDoor`) (`KismetMathLibrary.VLerp` _rightstartlocation (+ _rightstartlocation (0.0 -200.0 0.0)) _alpha) false false))))))

(event `self.ReceiveBeginPlay`
  (set `self.RightStartLocation` (`SceneComponent.K2_GetComponentLocation` (`self.RightDoor`)))
  (set `self.LeftStartLocation` (`SceneComponent.K2_GetComponentLocation` (`self.LeftDoor`))))

(fn `UserConstructionScript`)