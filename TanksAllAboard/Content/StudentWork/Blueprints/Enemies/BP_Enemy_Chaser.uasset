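; BP_Enemy_Chaser is an enemy that chases its target, commented as the player, and fires projectiles.
; Its Move event uses AI MoveTo toward MyTarget whenever that target is valid.
; Its Attack event calls HullToFace, then spawns a BP_EnemyProjectile at the FireArrow's location and rotation.
; The construction script only runs the parent's, and nothing in this graph triggers Move or Attack.
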(event `self.Move`
  (bind _mytarget (`self.MyTarget`))
  ;[1 1 1] Movement towards player
  (`/Engine/EditorBlueprintResources/StandardMacros.IsValid` _mytarget
    (:`Is Valid`
      (`|AIMoveTo` self (0.0 0.0 0.0) _mytarget))))

(event `self.Attack`
  (bind _firearrow (`self.FireArrow`))
  ;[0.4094 0 0.02868] Firing
  (`self.HullToFace`)
  (`|SpawnActorFromClass` "/Game/StudentWork/Blueprints/Projectiles/BP_EnemyProjectile.BP_EnemyProjectile_C" (`KismetMathLibrary.MakeTransform` (`SceneComponent.K2_GetComponentLocation` _firearrow) (`SceneComponent.K2_GetComponentRotation` _firearrow)) "Undefined" "MultiplyWithRoot" null null))

(fn `UserConstructionScript`
  (`parent.UserConstructionScript`))