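; Desert boss with three destructible phases: both hands, then both eyes, then the skull, whose death awards score and removes an invisible wall to open the arena exit.
; A timeline slides the skull between two points while a Delay in its update spawns fireballs aimed at the player at random intervals.
; Component hit events track health with flashing materials, camera shake and Niagara effects.
; Losing both eyes stops movement and firing, drops the skull and makes it vulnerable.
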(event `self.ReceiveBeginPlay`
  (bind _returnvalue (`GameplayStatics.GetPlayerCharacter` 0))
  (bind _handmaxhealth (`self.HandMaxHealth`))
  (bind _eyemaxhealth (`self.EyeMaxHealth`))
  (bind _startlocation (`self.StartLocation`))
  (bind _returnvalue_2 (`SceneComponent.K2_GetComponentLocation` (`self.FireballArrow`)))
  ;[0 0.9927 1] Setting Health Variables
  (set `self.RightHandCurrentHealth` _handmaxhealth)
  (set `self.LeftHandCurrentHealth` _handmaxhealth)
  (set `self.RightEyeCurrentHealth` _eyemaxhealth)
  (set `self.LeftEyeCurrentHealth` _eyemaxhealth)
  ;[0.0793 0 1] Makes hand targets flash
  (`PrimitiveComponent.SetMaterial` (`self.RightHandTarget`) 0 "/Game/StudentWork/Materials/M_Flashing_Inst1.M_Flashing_Inst1")
  (`PrimitiveComponent.SetMaterial` (`self.LeftHandTarget`) 0 "/Game/StudentWork/Materials/M_Flashing_Inst1.M_Flashing_Inst1")
  ;[1 0.5718 0] Skull Back and Forth Movement
  (set `self.StartLocation` (`SceneComponent.K2_GetComponentLocation` (`self.Skull`)))
  (bind (_direction _alpha) (`Timeline|TL_MainMovement` :!label _label)
    (:`Update`
      (if (`self.FinalAttackActivated`)
        (goto _label :!via `Stop`)
        (else
          (`SceneComponent.K2_SetWorldLocation` (`self.Skull`) (`KismetMathLibrary.VLerp` _startlocation (+ _startlocation (`self.OffsetLocation`)) _alpha) false false)
          ;[1 0 0.01044] Firing Projectiles
          (`KismetSystemLibrary.Delay` (`KismetMathLibrary.RandomFloatInRange` 0.3 2.5))
          (`/Engine/EditorBlueprintResources/StandardMacros.IsValid` _returnvalue
            (:`Is Valid`
              (`|SpawnActorFromClass` "/Game/StudentWork/Blueprints/Projectiles/BP_Fireball.BP_Fireball_C" (`KismetMathLibrary.MakeTransform` _returnvalue_2 (`KismetMathLibrary.FindLookAtRotation` _returnvalue_2 (`self.K2_GetActorLocation` _returnvalue))) "Undefined" "MultiplyWithRoot" null null))))))))

(event `self.RightHandTarget.OnComponentHit`
  (params (HitComponent :type "PrimitiveComponent Object Reference") (OtherActor :type "Actor Object Reference") (OtherComp :type "PrimitiveComponent Object Reference") (NormalImpulse :type "Vector Structure") (Hit :type "HitResult Structure (by ref)"))
  (bind _righthandtarget (`self.RightHandTarget`))
  ;[0.8959 0 1] Right Hand
  (set `self.RightHandCurrentHealth` (- (`self.RightHandCurrentHealth`) 20.0))
  (`PlayerCameraManager.StartCameraShake` :`self` (`GameplayStatics.GetPlayerCameraManager` 0) :`ShakeClass` "/Game/StudentWork/Blueprints/CS_DesertBossShake.CS_DesertBossShake_C" :`Scale` 1.5)
  (`PrimitiveComponent.SetMaterial` _righthandtarget 0 "/Game/StudentWork/Materials/M_EmissiveRed2.M_EmissiveRed2")
  (`KismetSystemLibrary.Delay` 0.5)
  (`PrimitiveComponent.SetMaterial` _righthandtarget 0 "/Game/StudentWork/Materials/M_Flashing_Inst1.M_Flashing_Inst1")
  (if (<= (`self.RightHandCurrentHealth`) 0.0)
    (`NiagaraFunctionLibrary.SpawnSystemAtLocation` "/Game/StudentWork/Systems/NS_Crumble3.NS_Crumble3" (`SceneComponent.K2_GetComponentLocation` (`self.RightHandTarget`)))
    (`KismetSystemLibrary.DelayUntilNextTick`)
    (`ActorComponent.K2_DestroyComponent` (`self.RightHandTarget`))
    (message `/Game/BI_score.I_UpdateScore` (`GameplayStatics.GetPlayerController` 0) 100.0)
    (bind _output_get (set `self.RightHandDestroyed` true))
    ;[1 1 1] Checks if both hands have been destroyed
    (if (and _output_get (stale `self.LeftHandTarget.OnComponentHit` _output_get)) :!label _label_2
      (set `self.EyesTargetsActivated` true)
      ;[0.06617 0 1] Makes eyes flash
      (`PrimitiveComponent.SetMaterial` (`self.RightEye`) 0 "/Game/StudentWork/Materials/M_Flashing_Inst1.M_Flashing_Inst1")
      (`PrimitiveComponent.SetMaterial` (`self.LeftEye`) 0 "/Game/StudentWork/Materials/M_Flashing_Inst1.M_Flashing_Inst1")
      (`KismetSystemLibrary.PrintString` "Hello"))))

(event `self.LeftHandTarget.OnComponentHit`
  (params (HitComponent :type "PrimitiveComponent Object Reference") (OtherActor :type "Actor Object Reference") (OtherComp :type "PrimitiveComponent Object Reference") (NormalImpulse :type "Vector Structure") (Hit :type "HitResult Structure (by ref)"))
  (bind _lefthandtarget (`self.LeftHandTarget`))
  ;[1 0.4218 0.9175] Left Hand
  (set `self.LeftHandCurrentHealth` (- (`self.LeftHandCurrentHealth`) 20.0))
  (`PlayerCameraManager.StartCameraShake` :`self` (`GameplayStatics.GetPlayerCameraManager` 0) :`ShakeClass` "/Game/StudentWork/Blueprints/CS_DesertBossShake.CS_DesertBossShake_C" :`Scale` 1.5)
  (`PrimitiveComponent.SetMaterial` _lefthandtarget 0 "/Game/StudentWork/Materials/M_EmissiveRed2.M_EmissiveRed2")
  (`KismetSystemLibrary.Delay` 0.5)
  (`PrimitiveComponent.SetMaterial` _lefthandtarget 0 "/Game/StudentWork/Materials/M_Flashing_Inst1.M_Flashing_Inst1")
  (if (<= (`self.LeftHandCurrentHealth`) 0.0)
    (`NiagaraFunctionLibrary.SpawnSystemAtLocation` "/Game/StudentWork/Systems/NS_Crumble3.NS_Crumble3" (`SceneComponent.K2_GetComponentLocation` (`self.LeftHandTarget`)))
    (`KismetSystemLibrary.DelayUntilNextTick`)
    (`ActorComponent.K2_DestroyComponent` (`self.LeftHandTarget`))
    (message `/Game/BI_score.I_UpdateScore` (`GameplayStatics.GetPlayerController` 0) 100.0)
    (bind _output_get (set `self.LeftHandDestroyed` true))
    (goto _label_2)))

(event `self.LeftEye.OnComponentHit`
  (params (HitComponent :type "PrimitiveComponent Object Reference") (OtherActor :type "Actor Object Reference") (OtherComp :type "PrimitiveComponent Object Reference") (NormalImpulse :type "Vector Structure") (Hit :type "HitResult Structure (by ref)"))
  (bind _lefteye (`self.LeftEye`))
  (bind _returnvalue (`SceneComponent.K2_GetComponentLocation` (`self.Skull`)))
  ;[1 0.2365 0.5505] Left Eye
  (if (`self.EyesTargetsActivated`)
    (set `self.LeftEyeCurrentHealth` (- (`self.LeftEyeCurrentHealth`) 20.0))
    (`PlayerCameraManager.StartCameraShake` :`self` (`GameplayStatics.GetPlayerCameraManager` 0) :`ShakeClass` "/Game/StudentWork/Blueprints/CS_DesertBossShake.CS_DesertBossShake_C" :`Scale` 1.5)
    (`PrimitiveComponent.SetMaterial` _lefteye 0 "/Game/StudentWork/Materials/M_EmissiveRed2.M_EmissiveRed2")
    (`KismetSystemLibrary.Delay` 0.5)
    (`PrimitiveComponent.SetMaterial` _lefteye 0 "/Game/StudentWork/Materials/M_Flashing_Inst1.M_Flashing_Inst1")
    (if (<= (`self.LeftEyeCurrentHealth`) 0.0)
      (`NiagaraFunctionLibrary.SpawnSystemAtLocation` "/Game/StudentWork/Systems/NS_Crumble3.NS_Crumble3" (`SceneComponent.K2_GetComponentLocation` (`self.LeftEye`)))
      (`KismetSystemLibrary.DelayUntilNextTick`)
      (`ActorComponent.K2_DestroyComponent` (`self.LeftEye`))
      (message `/Game/BI_score.I_UpdateScore` (`GameplayStatics.GetPlayerController` 0) 100.0)
      (bind _output_get (set `self.LeftEyeDestroyed` true))
      ;[1 1 1] Checks if both eyes have been destroyed
      (if (and _output_get (stale `self.RightEye.OnComponentHit` _output_get)) :!label _label_3
        (set `self.FinalAttackActivated` true)
        ;[0 1 0.6767] Fall
        (bind (_direction _alpha) (`Timeline|TL_Fall`)
          (:`Update`
            (`SceneComponent.K2_SetWorldLocation` (`self.Skull`) (`KismetMathLibrary.VLerp` _returnvalue (+ _returnvalue (0.0 0.0 -23.0)) _alpha) false false)))))))

(event `self.RightEye.OnComponentHit`
  (params (HitComponent :type "PrimitiveComponent Object Reference") (OtherActor :type "Actor Object Reference") (OtherComp :type "PrimitiveComponent Object Reference") (NormalImpulse :type "Vector Structure") (Hit :type "HitResult Structure (by ref)"))
  (bind _righteye (`self.RightEye`))
  ;[0.8885 0 0.3785] Right Eye
  (if (`self.EyesTargetsActivated`)
    (set `self.RightEyeCurrentHealth` (- (`self.RightEyeCurrentHealth`) 20.0))
    (`PlayerCameraManager.StartCameraShake` :`self` (`GameplayStatics.GetPlayerCameraManager` 0) :`ShakeClass` "/Game/StudentWork/Blueprints/CS_DesertBossShake.CS_DesertBossShake_C" :`Scale` 1.5)
    (`PrimitiveComponent.SetMaterial` _righteye 0 "/Game/StudentWork/Materials/M_EmissiveRed2.M_EmissiveRed2")
    (`KismetSystemLibrary.Delay` 0.5)
    (`PrimitiveComponent.SetMaterial` _righteye 0 "/Game/StudentWork/Materials/M_Flashing_Inst1.M_Flashing_Inst1")
    (if (<= (`self.RightEyeCurrentHealth`) 0.0)
      (`NiagaraFunctionLibrary.SpawnSystemAtLocation` "/Game/StudentWork/Systems/NS_Crumble3.NS_Crumble3" (`SceneComponent.K2_GetComponentLocation` (`self.RightEye`)))
      (`KismetSystemLibrary.DelayUntilNextTick`)
      (`ActorComponent.K2_DestroyComponent` (`self.RightEye`))
      (message `/Game/BI_score.I_UpdateScore` (`GameplayStatics.GetPlayerController` 0) 100.0)
      (bind _output_get (set `self.RightEyeDestroyed` true))
      (goto _label_3))))

(event `self.Skull.OnComponentHit`
  (params (HitComponent :type "PrimitiveComponent Object Reference") (OtherActor :type "Actor Object Reference") (OtherComp :type "PrimitiveComponent Object Reference") (NormalImpulse :type "Vector Structure") (Hit :type "HitResult Structure (by ref)"))
  (bind _skull (`self.Skull`))
  (bind _returnvalue (`SceneComponent.K2_GetComponentLocation` (`self.Skull`)))
  ;[1 0.1681 0] Final Attack
  (if (`self.FinalAttackActivated`)
    (set `self.FinalAttackHealth` (- (`self.FinalAttackHealth`) 20.0))
    (if (<= (`self.FinalAttackHealth`) 0.0)
      (`PlayerCameraManager.StartCameraShake` :`self` (`GameplayStatics.GetPlayerCameraManager` 0) :`ShakeClass` "/Game/StudentWork/Blueprints/CS_DesertBossShake.CS_DesertBossShake_C" :`Scale` 1.5)
      (`PrimitiveComponent.SetMaterial` _skull 0 "/Game/StudentWork/Materials/M_EmissiveRed2.M_EmissiveRed2")
      (`KismetSystemLibrary.Delay` 0.5)
      (`PrimitiveComponent.SetMaterial` _skull 0 "/Game/StudentWork/Materials/M_Flashing_Inst1.M_Flashing_Inst1")
      (`NiagaraFunctionLibrary.SpawnSystemAtLocation` "/Game/StudentWork/Systems/NS_Crumble.NS_Crumble" _returnvalue)
      (`NiagaraFunctionLibrary.SpawnSystemAtLocation` "/Game/StudentWork/Systems/NS_Confetti.NS_Confetti" _returnvalue)
      (`self.K2_DestroyActor`)
      (message `/Game/BI_score.I_UpdateScore` (`GameplayStatics.GetPlayerController` 0) 1000.0)
      ;[0.3925 1 0.9622] Allows player to exit arena
      (`self.K2_DestroyActor` (`self.InvisibleWall`)))))

(fn `UserConstructionScript`)