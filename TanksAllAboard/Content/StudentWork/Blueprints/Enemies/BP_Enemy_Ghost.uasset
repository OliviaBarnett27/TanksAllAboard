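; Ghost enemy that blinks around a fixed rectangular area, damaging the player and affecting score.
; An endless BeginPlay delay loop reveals the mesh at a random XY position at unchanged height, then hides it again.
; Mesh overlap with the player applies damage and a score penalty.
; Any mesh hit lowers ghost health, destroying it at zero and awarding points through the player controller's interface.
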(event `self.ReceiveBeginPlay`
  (bind (_returnvalue_x _returnvalue_y _returnvalue_z) (`KismetMathLibrary.BreakVector` (`SceneComponent.K2_GetComponentLocation` (`self.CapsuleComponent`))))
  ;[1 1 1] Controls location and movement of ghosts
  (`KismetSystemLibrary.Delay` (`KismetMathLibrary.RandomFloatInRange` 0.3 0.7) :!label _label)
  (`SceneComponent.SetHiddenInGame` (`self.StaticMesh`) false false)
  (`SceneComponent.K2_SetWorldLocation` (`self.CapsuleComponent`) (`KismetMathLibrary.MakeVector` (`KismetMathLibrary.RandomFloatInRange` 7290.0 12090.0) (`KismetMathLibrary.RandomFloatInRange` 46210.0 53210.0) _returnvalue_z) false false)
  (`KismetSystemLibrary.Delay` 0.5)
  (`SceneComponent.SetHiddenInGame` (`self.StaticMesh`) true false)
  (goto _label))

(event `self.StaticMesh.OnComponentBeginOverlap`
  (params (OverlappedComponent :type "PrimitiveComponent Object Reference") (OtherActor :type "Actor Object Reference") (OtherComp :type "PrimitiveComponent Object Reference") (OtherBodyIndex :type Integer) (bFromSweep :type Boolean) (SweepResult :type "HitResult Structure (by ref)"))
  ;[1 1 1] Damage player and adjust score
  (bind _asbp_player_character (cast `/Game/Blueprints/BP_PlayerCharacter` OtherActor))
  (`GameplayStatics.ApplyDamage` _asbp_player_character 10.0)
  (message `/Game/BI_score.I_UpdateScore` (`GameplayStatics.GetPlayerController` 0) -50.0))

(event `self.StaticMesh.OnComponentHit`
  (params (HitComponent :type "PrimitiveComponent Object Reference") (OtherActor :type "Actor Object Reference") (OtherComp :type "PrimitiveComponent Object Reference") (NormalImpulse :type "Vector Structure") (Hit :type "HitResult Structure (by ref)"))
  ;[1 0 0.05077] Ghost Damage
  (set `self.GhostHealth` (- (`self.GhostHealth`) 5.0))
  (if (<= (`self.GhostHealth`) 0.0)
    (`self.K2_DestroyActor`)
    (message `/Game/BI_score.I_UpdateScore` (`GameplayStatics.GetPlayerController` 0) 250.0)))

(fn `UserConstructionScript`)