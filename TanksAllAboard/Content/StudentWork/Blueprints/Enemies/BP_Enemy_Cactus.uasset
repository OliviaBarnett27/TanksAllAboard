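; Cactus enemy that starts with its face hidden, then reveals it and chases the player once they enter its detection sphere.
; A looping timer reissues AI MoveTo and swaps the mesh material; HullToFace eases rotation toward velocity but is not called in this graph.
; Capsule overlap damages the player and deducts score, gated by a short cooldown.
; Any mesh hit drains health, destroying the cactus at zero and awarding score through the player controller.
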(event `self.ReceiveBeginPlay`
  ;[1 1 1] Hide Face
  (`SceneComponent.SetHiddenInGame` (`self.Mouth`) true false)
  (`SceneComponent.SetHiddenInGame` (`self.REyebrow`) true false)
  (`SceneComponent.SetHiddenInGame` (`self.LeftEye`) true false)
  (`SceneComponent.SetHiddenInGame` (`self.LEyebrow`) true false)
  (`SceneComponent.SetHiddenInGame` (`self.RightEye`) true false))

(event `StartCactusMovementTimer`
  ;[1 1 1] Movement Timer
  (bind _returnvalue (`KismetSystemLibrary.K2_SetTimerDelegate` (delegate `CactusMovement`) 1.0 true))
  (set `self.Timer` _returnvalue))

(event `HullToFace`
  (bind _staticmesh (`self.StaticMesh`))
  (bind (_returnvalue_roll _returnvalue_pitch _returnvalue_yaw) (`KismetMathLibrary.BreakRotator` (`KismetMathLibrary.MakeRotFromX` (`self.GetVelocity`))))
  ;[1 1 1] Rotates the cactus model over time to look in direction it's moving
  (`SceneComponent.K2_SetWorldRotation` _staticmesh (`KismetMathLibrary.RInterpTo` (`SceneComponent.K2_GetComponentRotation` _staticmesh) (`KismetMathLibrary.MakeRotator` 0.0 0.0 _returnvalue_yaw) (`GameplayStatics.GetWorldDeltaSeconds`) 2.0) false false))

(event `CactusMovement`
  ;[1 1 1] Movement Timer
  ;[1 1 1] Makes the cactus look like an enemy (changes material and unhides face)
  (`PrimitiveComponent.SetMaterial` (`self.StaticMesh`) 0 "/Game/StudentWork/Materials/M_Material1_Inst.M_Material1_Inst")
  (`SceneComponent.SetHiddenInGame` (`self.Mouth`) false false)
  (`SceneComponent.SetHiddenInGame` (`self.REyebrow`) false false)
  (`SceneComponent.SetHiddenInGame` (`self.LeftEye`) false false)
  (`SceneComponent.SetHiddenInGame` (`self.LEyebrow`) false false)
  (`SceneComponent.SetHiddenInGame` (`self.RightEye`) false false)
  ;[1 1 1] Movement to chase player
  (`|AIMoveTo` self (0.0 0.0 0.0) (`GameplayStatics.GetPlayerCharacter` 0) 1.0))

(event `self.SphereCollision.OnComponentBeginOverlap`
  (params (OverlappedComponent :type "PrimitiveComponent Object Reference") (OtherActor :type "Actor Object Reference") (OtherComp :type "PrimitiveComponent Object Reference") (OtherBodyIndex :type Integer) (bFromSweep :type Boolean) (SweepResult :type "HitResult Structure (by ref)"))
  ;[1 1 1] Activates when the player enters the collision detection radius
  (cast `/Game/Blueprints/BP_PlayerCharacter` OtherActor)
  (`KismetSystemLibrary.Delay` 0.2)
  (`self.StartCactusMovementTimer`))

(event `self.Capsule.OnComponentBeginOverlap`
  (params (OverlappedComponent :type "PrimitiveComponent Object Reference") (OtherActor :type "Actor Object Reference") (OtherComp :type "PrimitiveComponent Object Reference") (OtherBodyIndex :type Integer) (bFromSweep :type Boolean) (SweepResult :type "HitResult Structure (by ref)"))
  ;[1 1 1] Apply Damage
  (bind _asbp_player_character (cast `/Game/Blueprints/BP_PlayerCharacter` OtherActor))
  (if (not (`self.IsDamageCooldown?`))
    (`GameplayStatics.ApplyDamage` _asbp_player_character 10.0)
    ;[1 1 1] Adjust player score
    (message `/Game/BI_score.I_UpdateScore` (`GameplayStatics.GetPlayerController` 0) -75.0)
    ;[1 1 1] Damage cooldown
    (set `self.IsDamageCooldown?` true)
    (`KismetSystemLibrary.K2_SetTimerDelegate` (delegate `EndDamgeCooldown`) 0.3)))

(event `EndDamgeCooldown`
  ;[1 1 1] Damage cooldown
  (set `self.IsDamageCooldown?` false))

(event `self.StaticMesh.OnComponentHit`
  (params (HitComponent :type "PrimitiveComponent Object Reference") (OtherActor :type "Actor Object Reference") (OtherComp :type "PrimitiveComponent Object Reference") (NormalImpulse :type "Vector Structure") (Hit :type "HitResult Structure (by ref)"))
  ;[1 1 1] Destroyed when shot by the player
  (`KismetSystemLibrary.PrintString` "Hello")
  (bind _output_get (set `self.CactusHealth` (- (`self.CactusHealth`) 20.0)))
  (if (<= _output_get 0.0)
    (`self.K2_DestroyActor`)
    (message `/Game/BI_score.I_UpdateScore` (`GameplayStatics.GetPlayerController` 0) 150.0)))

(fn `UserConstructionScript`)