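; BP_Enemy_MoveRandom is an enemy pawn variant that wanders at random and fires projectiles.
; Its Move event sends the pawn via AI MoveTo to a random reachable navmesh point within a fixed radius of its current location.
; Its Attack event calls HullToFace, then spawns a BP_EnemyProjectile at the FireArrow's world location and rotation.
; The construction script only runs the parent's.
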(event `self.Move`
  ;[0 0.8856 1] Movement
  (`|AIMoveTo` self (`NavigationSystemV1.K2_GetRandomReachablePointInRadius` (`self.K2_GetActorLocation`) 600.0 null null) null))

(event `self.Attack`
  (bind _firearrow (`self.FireArrow`))
  ;[0.4094 0 0.02868] Firing
  (`self.HullToFace`)
  (`|SpawnActorFromClass` "/Game/StudentWork/Blueprints/Projectiles/BP_EnemyProjectile.BP_EnemyProjectile_C" (`KismetMathLibrary.MakeTransform` (`SceneComponent.K2_GetComponentLocation` _firearrow) (`SceneComponent.K2_GetComponentRotation` _firearrow)) "Undefined" "MultiplyWithRoot" null null))

(fn `UserConstructionScript`
  (`parent.UserConstructionScript`))