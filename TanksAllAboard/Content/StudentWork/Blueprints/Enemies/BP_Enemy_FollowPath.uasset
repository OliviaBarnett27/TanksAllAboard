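; Enemy pawn that makes a short scripted move along the Y axis and can fire projectiles.
; On BeginPlay, Move issues an AI move 500 units toward -Y, then one second later issues one 500 units toward +Y from its current location.
; The second move waits on a timer, not arrival, and the sequence does not loop.
; Attack calls HullToFace and spawns BP_EnemyProjectile at the FireArrow transform.
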(event `self.Move`
  ;[0 0.9592 1] Movement
  (`|AIMoveTo` self (+ (`self.K2_GetActorLocation`) (0.0 -500.0 0.0)) null
    (:`then`
      (`KismetSystemLibrary.Delay` 1.0)
      (`|AIMoveTo` self (+ (`self.K2_GetActorLocation`) (0.0 500.0 0.0)) null
        (:`then`
          (`KismetSystemLibrary.Delay` 1.0))))))

(event `self.Attack`
  (bind _firearrow (`self.FireArrow`))
  ;[0.4094 0 0.02868] Firing
  (`self.HullToFace`)
  (`|SpawnActorFromClass` "/Game/StudentWork/Blueprints/Projectiles/BP_EnemyProjectile.BP_EnemyProjectile_C" (`KismetMathLibrary.MakeTransform` (`SceneComponent.K2_GetComponentLocation` _firearrow) (`SceneComponent.K2_GetComponentRotation` _firearrow)) "Undefined" "MultiplyWithRoot" null null))

(event `self.ReceiveBeginPlay`
  (`self.Move`))

(fn `UserConstructionScript`
  (`parent.UserConstructionScript`))