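; Ghost boss enemy that teleports around a fixed arena, attacks with projectiles and explosives, and damages the player on overlap, costing them score.
; A looping delay chain from BeginPlay moves it to a random spot, reveals it, spawns a delayed random explosive, fires eight-arrow volleys in threes while stepping Sphere yaw, then hides it.
; Any mesh hit lowers its health; death spawns crumble VFX, destroys it and awards score.
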(event `self.StaticMesh.OnComponentBeginOverlap`
  (params (OverlappedComponent :type "PrimitiveComponent Object Reference") (OtherActor :type "Actor Object Reference") (OtherComp :type "PrimitiveComponent Object Reference") (OtherBodyIndex :type Integer) (bFromSweep :type Boolean) (SweepResult :type "HitResult Structure (by ref)"))
  ;[1 1 1] Cause damage to player and adjust score
  (bind _asbp_player_character (cast `/Game/Blueprints/BP_PlayerCharacter` OtherActor))
  (`GameplayStatics.ApplyDamage` _asbp_player_character 10.0)
  (message `/Game/BI_score.I_UpdateScore` (`GameplayStatics.GetPlayerController` 0) -50.0))

(event `self.ReceiveBeginPlay`
  (bind _sphere (`self.Sphere`))
  (bind (_returnvalue_roll _returnvalue_pitch _returnvalue_yaw) (`KismetMathLibrary.BreakRotator` (`SceneComponent.K2_GetComponentRotation` _sphere)))
  (bind (_returnvalue_x _returnvalue_y _returnvalue_z) (`KismetMathLibrary.BreakVector` (`SceneComponent.K2_GetComponentLocation` (`self.BoxCollision`))))
  ;[0.1778 0.5333 1] Sets location of boss
  (set `self.Z` (+ _returnvalue_z -200.0))
  (`KismetSystemLibrary.Delay` (`KismetMathLibrary.RandomFloatInRange` 0.7 1.0) :!label _label)
  (`SceneComponent.K2_SetWorldLocation` (`self.CapsuleComponent`) (`KismetMathLibrary.MakeVector` (`KismetMathLibrary.RandomFloatInRange` 15247.0 18202.0) (`KismetMathLibrary.RandomFloatInRange` 48332.0 51062.0) (`self.Z`)) false false)
  (`SceneComponent.SetHiddenInGame` (`self.StaticMesh`) false false)
  (`self.SpawnExplosive`)
  (`KismetSystemLibrary.Delay` 0.5)
  ;[0.8719 0.2131 0] When projectiles are shot
  (`KismetSystemLibrary.Delay` (`KismetMathLibrary.RandomFloatInRange` 0.3 1.5))
  ;[1 0.2519 0] Shoots projectiles in threes
  (for _ (range 3)
    (`SceneComponent.K2_SetWorldRotation` _sphere (`KismetMathLibrary.MakeRotator` 0.0 0.0 (+ _returnvalue_yaw 10.0)) false false)
    (`self.Shoot Projectiles`)
    ;[1 1 1] Hides boss
    (`SceneComponent.SetHiddenInGame` (`self.StaticMesh`) true false)
    (goto _label)))

(event `self.StaticMesh.OnComponentHit`
  (params (HitComponent :type "PrimitiveComponent Object Reference") (OtherActor :type "Actor Object Reference") (OtherComp :type "PrimitiveComponent Object Reference") (NormalImpulse :type "Vector Structure") (Hit :type "HitResult Structure (by ref)"))
  ;[1 0 0.001667] Damage
  (set `self.GhostHealth` (- (`self.GhostHealth`) 10.0))
  (if (<= (`self.GhostHealth`) 0.0)
    (`PrimitiveComponent.SetMaterial` (`self.StaticMesh`) 0 "/Game/StudentWork/Materials/M_Flashing_Inst2.M_Flashing_Inst2")
    (`NiagaraFunctionLibrary.SpawnSystemAtLocation` "/Game/StudentWork/Systems/NS_Crumble4.NS_Crumble4")
    (`self.K2_DestroyActor`)
    (message `/Game/BI_score.I_UpdateScore` (`GameplayStatics.GetPlayerController` 0) 1000.0)))

(event `SpawnExplosive`
  ;[1 1 1] Spawn explosives
  (`KismetSystemLibrary.Delay` (`KismetMathLibrary.RandomFloatInRange` 1.0 2.0))
  (`|SpawnActorFromClass` "/Game/StudentWork/Blueprints/BP_GhostExplosive.BP_GhostExplosive_C" (`KismetMathLibrary.MakeTransform` (`KismetMathLibrary.MakeVector` (`KismetMathLibrary.RandomFloatInRange` 15247.0 18202.0) (`KismetMathLibrary.RandomFloatInRange` 48332.0 51062.0) (+ (`self.Z`) 300.0))) "Undefined" "MultiplyWithRoot" null null))

(event `Shoot Projectiles`
  (bind (_returnvalue_location _returnvalue_rotation) (`KismetMathLibrary.BreakTransform` (`SceneComponent.K2_GetComponentToWorld` (`self.Arrow3`))))
  (bind (_returnvalue_location_2 _returnvalue_rotation_2) (`KismetMathLibrary.BreakTransform` (`SceneComponent.K2_GetComponentToWorld` (`self.Arrow1`))))
  (bind (_returnvalue_location_3 _returnvalue_rotation_3) (`KismetMathLibrary.BreakTransform` (`SceneComponent.K2_GetComponentToWorld` (`self.Arrow2`))))
  (bind (_returnvalue_location_4 _returnvalue_rotation_4) (`KismetMathLibrary.BreakTransform` (`SceneComponent.K2_GetComponentToWorld` (`self.Arrow8`))))
  (bind (_returnvalue_location_5 _returnvalue_rotation_5) (`KismetMathLibrary.BreakTransform` (`SceneComponent.K2_GetComponentToWorld` (`self.Arrow6`))))
  (bind (_returnvalue_location_6 _returnvalue_rotation_6) (`KismetMathLibrary.BreakTransform` (`SceneComponent.K2_GetComponentToWorld` (`self.Arrow5`))))
  (bind (_returnvalue_location_7 _returnvalue_rotation_7) (`KismetMathLibrary.BreakTransform` (`SceneComponent.K2_GetComponentToWorld` (`self.Arrow4`))))
  (bind (_returnvalue_location_8 _returnvalue_rotation_8) (`KismetMathLibrary.BreakTransform` (`SceneComponent.K2_GetComponentToWorld` (`self.Arrow7`))))
  ;[1 0.2636 0] Projectiles
  (`|SpawnActorFromClass` "/Game/StudentWork/Blueprints/Projectiles/BP_GhostBalls.BP_GhostBalls_C" (`KismetMathLibrary.MakeTransform` _returnvalue_location_2 _returnvalue_rotation_2) "Undefined" "MultiplyWithRoot" null null)
  (`|SpawnActorFromClass` "/Game/StudentWork/Blueprints/Projectiles/BP_GhostBalls.BP_GhostBalls_C" (`KismetMathLibrary.MakeTransform` _returnvalue_location_3 _returnvalue_rotation_3) "Undefined" "MultiplyWithRoot" null null)
  (`|SpawnActorFromClass` "/Game/StudentWork/Blueprints/Projectiles/BP_GhostBalls.BP_GhostBalls_C" (`KismetMathLibrary.MakeTransform` _returnvalue_location _returnvalue_rotation) "Undefined" "MultiplyWithRoot" null null)
  (`|SpawnActorFromClass` "/Game/StudentWork/Blueprints/Projectiles/BP_GhostBalls.BP_GhostBalls_C" (`KismetMathLibrary.MakeTransform` _returnvalue_location_7 _returnvalue_rotation_7) "Undefined" "MultiplyWithRoot" null null)
  (`|SpawnActorFromClass` "/Game/StudentWork/Blueprints/Projectiles/BP_GhostBalls.BP_GhostBalls_C" (`KismetMathLibrary.MakeTransform` _returnvalue_location_6 _returnvalue_rotation_6) "Undefined" "MultiplyWithRoot" null null)
  (`|SpawnActorFromClass` "/Game/StudentWork/Blueprints/Projectiles/BP_GhostBalls.BP_GhostBalls_C" (`KismetMathLibrary.MakeTransform` _returnvalue_location_5 _returnvalue_rotation_5) "Undefined" "MultiplyWithRoot" null null)
  (`|SpawnActorFromClass` "/Game/StudentWork/Blueprints/Projectiles/BP_GhostBalls.BP_GhostBalls_C" (`KismetMathLibrary.MakeTransform` _returnvalue_location_8 _returnvalue_rotation_8) "Undefined" "MultiplyWithRoot" null null)
  (`|SpawnActorFromClass` "/Game/StudentWork/Blueprints/Projectiles/BP_GhostBalls.BP_GhostBalls_C" (`KismetMathLibrary.MakeTransform` _returnvalue_location_4 _returnvalue_rotation_4) "Undefined" "MultiplyWithRoot" null null))

(fn `UserConstructionScript`)