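; Enemy actor that starts out friendly or hostile based on IsEnemy; damaging a friendly one turns it hostile.
; The first hit on a friendly flashes the weapon detail's dynamic material via timeline, then swaps the body to red.
; A hit while hostile flashes, applies damage, and at zero health awards score and destroys the actor.
; Attack turns the hull and fires a projectile from FireArrow only while hostile.
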(event `self.ReceiveAnyDamage`
  (params (Damage :type "Float (single-precision)") (DamageType :type "DamageType Object Reference") (InstigatedBy :type "Controller Object Reference") (DamageCauser :type "Actor Object Reference"))
  (if (`self.IsEnemy?`)
    ;[1 0 0.03162] Enemy
    (`/Engine/EditorBlueprintResources/StandardMacros.DoOnce` false
      (:`Completed`
        (bind (_direction _flash) (`Timeline|TL_DestroyedFlash` :!via `PlayFromStart`)
          (:`Update`
            (`MaterialInstanceDynamic.SetScalarParameterValue` (`self.Flashing Material`) "FlashLevel" _flash))
          (:`Finished`
            (bind _returnvalue (`GameplayStatics.ApplyDamage` null))
            (set `self.CurrentHealth` _returnvalue)
            (if (<= (`self.CurrentHealth`) 0.0)
              (`self.K2_DestroyActor`)
              (message `/Game/BI_score.I_UpdateScore` (`GameplayStatics.GetPlayerController` 0) 250.0)
              (`self.K2_DestroyActor`))))))
    (else
      ;[0.1984 1 0.1714] Friendly
      (`/Engine/EditorBlueprintResources/StandardMacros.DoOnce` false
        (:`Completed`
          (bind (_direction_2 _flash_2) (`Timeline|TL_ChangeToEnemyFlash` :!via `PlayFromStart`)
            (:`Update`
              (`MaterialInstanceDynamic.SetScalarParameterValue` (`self.Flashing Material`) "FlashLevel" _flash_2))
            (:`Finished`
              (`PrimitiveComponent.SetMaterial` (`self.Body`) 0 "/Game/Materials/M_SciFi_Red.M_SciFi_Red")
              (set `self.IsEnemy?` true))))))))

(event `self.Attack`
  (bind (_returnvalue_location _returnvalue_rotation) (`KismetMathLibrary.BreakTransform` (`SceneComponent.K2_GetComponentToWorld` (`self.FireArrow`))))
  ;[0.7302 0 0.1071] Fire
  (if (`self.IsEnemy?`)
    (`self.HullToFace`)
    (`|SpawnActorFromClass` "/Game/StudentWork/Blueprints/Projectiles/BP_EnemyProjectile.BP_EnemyProjectile_C" (`KismetMathLibrary.MakeTransform` _returnvalue_location _returnvalue_rotation) "Undefined" "MultiplyWithRoot" null null)))

(fn `UserConstructionScript`
  (`parent.UserConstructionScript`)
  (bind _returnvalue (`PrimitiveComponent.CreateDynamicMaterialInstance` (`self.WeaponDetail`) 0 "/Game/StudentWork/Materials/M_ControlledFlash_Inst.M_ControlledFlash_Inst" "None"))
  (set `self.Flashing Material` _returnvalue))