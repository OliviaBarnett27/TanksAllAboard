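; BP_GhostExplosive is a short-lived explosive actor that damages the player character when it detonates.
; BeginPlay attaches a spawn effect to its StaticMesh and starts a fuse, while a mesh hit starts a shorter delay into the same detonation.
; Detonation plays an upward mesh burst, calls ApplyDamage on player 0 with no distance or overlap check, then destroys the actor.
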(event `self.ReceiveBeginPlay`
  (`NiagaraFunctionLibrary.SpawnSystemAttached` "/Game/StudentWork/Systems/NS_Spawn.NS_Spawn" (`self.StaticMesh`) "None" (0.0 0.0 0.0) (struct) "KeepRelativeOffset")
  (`KismetSystemLibrary.Delay` 1.5)
  (`NiagaraFunctionLibrary.SpawnSystemAtLocation` "/Game/StudentWork/Systems/NS_UpwardMeshBurst.NS_UpwardMeshBurst" (`SceneComponent.K2_GetComponentLocation` (`self.StaticMesh`)) :!label _label)
  (`GameplayStatics.ApplyDamage` (`GameplayStatics.GetPlayerCharacter` 0))
  (`self.K2_DestroyActor`))

(event `self.StaticMesh.OnComponentHit`
  (params (HitComponent :type "PrimitiveComponent Object Reference") (OtherActor :type "Actor Object Reference") (OtherComp :type "PrimitiveComponent Object Reference") (NormalImpulse :type "Vector Structure") (Hit :type "HitResult Structure (by ref)"))
  (`KismetSystemLibrary.Delay` 0.2)
  (goto _label))

(fn `UserConstructionScript`)