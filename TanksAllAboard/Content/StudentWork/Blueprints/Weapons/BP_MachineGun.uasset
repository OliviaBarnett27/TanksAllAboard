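; BP_MachineGun is a tank weapon that fires a rapid spread of machine gun projectiles from the owning tank.
; Each trigger spawns three BP_MachineGunPlayerProjectile actors at the tank's DirectionArrow, one centered and two at opposite diagonal world-space offsets, all sharing the arrow's rotation.
; A Cooldown flag, cleared by a short non-looping timer, limits the fire rate.
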(event `self.Triggered`
  (bind _directionarrow (`/Game/Blueprints/BP_PlayerCharacter.DirectionArrow` (`self.MyTank`)))
  (bind _returnvalue (`SceneComponent.K2_GetComponentLocation` _directionarrow))
  (bind _returnvalue_2 (`SceneComponent.K2_GetComponentRotation` _directionarrow))
  (if (not (`self.Cooldown`))
    (`|SpawnActorFromClass` "/Game/StudentWork/Blueprints/Projectiles/BP_MachineGunPlayerProjectile.BP_MachineGunPlayerProjectile_C" (`KismetMathLibrary.MakeTransform` _returnvalue _returnvalue_2) "Undefined" "MultiplyWithRoot" null null)
    (`|SpawnActorFromClass` "/Game/StudentWork/Blueprints/Projectiles/BP_MachineGunPlayerProjectile.BP_MachineGunPlayerProjectile_C" (`KismetMathLibrary.MakeTransform` (+ _returnvalue (-10.0 -10.0 -10.0)) _returnvalue_2) "Undefined" "MultiplyWithRoot" null null)
    (`|SpawnActorFromClass` "/Game/StudentWork/Blueprints/Projectiles/BP_MachineGunPlayerProjectile.BP_MachineGunPlayerProjectile_C" (`KismetMathLibrary.MakeTransform` (+ _returnvalue (10.0 10.0 10.0)) _returnvalue_2) "Undefined" "MultiplyWithRoot" null null)
    (set `self.Cooldown` true)
    (`KismetSystemLibrary.K2_SetTimerDelegate` (delegate `End Cooldown`) 0.075)))

(event `End Cooldown`
  (set `self.Cooldown` false))

(fn `UserConstructionScript`
  (`parent.UserConstructionScript`))