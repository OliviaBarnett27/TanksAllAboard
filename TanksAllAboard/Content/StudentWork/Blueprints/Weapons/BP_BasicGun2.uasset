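; BP_BasicGun2 is a basic tank weapon that fires a player projectile when triggered.
; Triggered spawns BP_BasicGun_PlayerProjectile at the location and rotation of the owning tank's DirectionArrow, reached through MyTank.
; A Cooldown flag blocks further shots until a short one-shot timer calls EndCooldown to clear it, limiting the fire rate.
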(event `self.Triggered`
  (bind _directionarrow (`/Game/Blueprints/BP_PlayerCharacter.DirectionArrow` (`self.MyTank`)))
  (if (not (`self.Cooldown`))
    (`|SpawnActorFromClass` "/Game/StudentWork/Blueprints/Projectiles/BP_BasicGun_PlayerProjectile.BP_BasicGun_PlayerProjectile_C" (`KismetMathLibrary.MakeTransform` (`SceneComponent.K2_GetComponentLocation` _directionarrow) (`SceneComponent.K2_GetComponentRotation` _directionarrow)) "Undefined" "MultiplyWithRoot" null null)
    (set `self.Cooldown` true)
    (`KismetSystemLibrary.K2_SetTimerDelegate` (delegate `End Cooldown`) 0.3)))

(event `End Cooldown`
  (set `self.Cooldown` false))

(fn `UserConstructionScript`
  (`parent.UserConstructionScript`))