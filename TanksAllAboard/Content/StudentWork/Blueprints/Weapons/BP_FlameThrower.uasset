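; Flamethrower weapon that fires from the tank's direction arrow and damages actors close to it.
; Started spawns an attached Niagara flame effect, and Completed deactivates it.
; While triggered, a multi-sphere object trace at the arrow applies damage to each hit, rate-limited by a short cooldown timer.
; The trace's forward offset is multiplied by zero, so it covers only a sphere around the arrow.
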(event `self.Started`
  (bind _returnvalue (`NiagaraFunctionLibrary.SpawnSystemAttached` "/Game/StudentWork/Systems/NS_Flamer.NS_Flamer" (`/Game/Blueprints/BP_PlayerCharacter.DirectionArrow` (`self.MyTank`)) "None" (0.0 0.0 0.0) (struct) "KeepRelativeOffset"))
  (set `self.Flame System` _returnvalue))

(event `self.Completed`
  (`ActorComponent.Deactivate` (`self.Flame System`)))

(event `self.Triggered`
  (bind _directionarrow (`/Game/Blueprints/BP_PlayerCharacter.DirectionArrow` (`self.MyTank`)))
  (bind _returnvalue_location (`KismetMathLibrary.BreakTransform` (`SceneComponent.K2_GetComponentToWorld` _directionarrow)))
  (if (not (`self.Cooldown`))
    (bind _outhits (`KismetSystemLibrary.SphereTraceMultiForObjects` _returnvalue_location (+ _returnvalue_location (* (`SceneComponent.GetForwardVector` _directionarrow) (0.0 0.0 0.0))) 100.0 (`self.Object Types`)))
    (for _array_element _outhits
      (`GameplayStatics.ApplyDamage` (`.HitActor` (`GameplayStatics.BreakHitResult` _array_element)) 100.0))
    (set `self.Cooldown` true)
    (`KismetSystemLibrary.K2_SetTimerDelegate` (delegate `End Cooldown`) 0.2)))

(event `End Cooldown`
  (set `self.Cooldown` false))

(fn `UserConstructionScript`
  (`parent.UserConstructionScript`))