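; Train actor that starts moving once something first overlaps its base collision and stops near an offset from its start location.
; A fast looping timer nudges the mesh along its initial forward vector and spins four wheel roots until it arrives.
; Reset stops the timer, returns the mesh to the start and re-arms the trigger for respawns.
; CrashEffect provides a camera shake and brief white fade, with no caller in this graph.
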(event `self.Base Collision.OnComponentBeginOverlap`
  (params (OverlappedComponent :type "PrimitiveComponent Object Reference") (OtherActor :type "Actor Object Reference") (OtherComp :type "PrimitiveComponent Object Reference") (OtherBodyIndex :type Integer) (bFromSweep :type Boolean) (SweepResult :type "HitResult Structure (by ref)"))
  ;[1 1 1] Begins movement
  (`/Engine/EditorBlueprintResources/StandardMacros.DoOnce` false :!label _label
    (:`Completed`
      (bind _returnvalue (`KismetSystemLibrary.K2_SetTimerDelegate` (delegate `Move`) 0.001 true))
      (set `self.MovementTimer` _returnvalue))))

(event `Move`
  ;[1 1 1] Begins movement
  (`SceneComponent.K2_AddRelativeLocation` (`self.SM_Base`) (`self.ForwardVector`) true true)
  (if (< (`KismetMathLibrary.Vector_Distance` (`self.K2_GetActorLocation`) (+ (`self.StartLocation`) (`self.OffsetLocation`))) 10.0)
    ;[1 1 1] Resets timer
    (`KismetSystemLibrary.K2_ClearAndInvalidateTimerHandle` (`self.MovementTimer`))
    (else
      ;[1 1 1] Wheel rotation
      (`SceneComponent.K2_AddLocalRotation` (`self.WheelRoot`) (`KismetMathLibrary.MakeRotator` 0.0 1.0) false false)
      (`SceneComponent.K2_AddLocalRotation` (`self.WheelRoot1`) (`KismetMathLibrary.MakeRotator` 0.0 1.0) false false)
      (`SceneComponent.K2_AddLocalRotation` (`self.WheelRoot2`) (`KismetMathLibrary.MakeRotator` 0.0 1.0) false false)
      (`SceneComponent.K2_AddLocalRotation` (`self.WheelRoot3`) (`KismetMathLibrary.MakeRotator` 0.0 1.0) false false))))

(event `Reset`
  ;[1 1 1] Allows the train to return to its start location on respawn
  (`KismetSystemLibrary.K2_ClearAndInvalidateTimerHandle` (`self.MovementTimer`))
  (`SceneComponent.K2_SetWorldLocation` (`self.SM_Base`) (`self.StartLocation`) false false)
  (goto _label :!via `Reset`))

(event `self.ReceiveBeginPlay`
  ;[1 1 1] Setting variables
  (set `self.StartLocation` (`self.K2_GetActorLocation`))
  (set `self.ForwardVector` (`SceneComponent.GetForwardVector` (`self.SM_Base`))))

(fn `CrashEffect`
  (bind _returnvalue (`GameplayStatics.GetPlayerCameraManager` 0))
  (`PlayerCameraManager.StartCameraShake` :`self` _returnvalue :`Scale` 20.0)
  (`PlayerCameraManager.StartCameraFade` _returnvalue 0.0 0.1 0.15 (struct :`R` 1.0 :`G` 1.0 :`B` 1.0 :`A` 1.0) false false))

(fn `UserConstructionScript`)