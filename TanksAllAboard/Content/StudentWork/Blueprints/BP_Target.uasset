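; BP_Target is a damageable target actor that flashes, bursts and awards score when hit.
; The construction script creates a dynamic flash material on the static mesh.
; The first damage event, gated by DoOnce, plays a timeline that drives the material's FlashLevel parameter.
; When the timeline finishes, it spawns an upward mesh burst, sends points to the player controller through a score message and destroys itself.
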(event `self.ReceiveAnyDamage`
  (params (Damage :type "Float (single-precision)") (DamageType :type "DamageType Object Reference") (InstigatedBy :type "Controller Object Reference") (DamageCauser :type "Actor Object Reference"))
  (`/Engine/EditorBlueprintResources/StandardMacros.DoOnce` false
    (:`Completed`
      (bind (_direction _flash) (`Timeline|TL_Flash` :!via `PlayFromStart`)
        (:`Update`
          (`MaterialInstanceDynamic.SetScalarParameterValue` (`self.Flash Material`) "FlashLevel" _flash))
        (:`Finished`
          (`NiagaraFunctionLibrary.SpawnSystemAtLocation` "/Game/StudentWork/Systems/NS_UpwardMeshBurst.NS_UpwardMeshBurst" (`SceneComponent.K2_GetComponentLocation` (`self.StaticMesh`)))
          (set `self.Explosion` null)
          (message `/Game/BI_score.I_UpdateScore` (`GameplayStatics.GetPlayerController` 0) 100.0)
          (`self.K2_DestroyActor`))))))

(fn `UserConstructionScript`
  (bind _returnvalue (`PrimitiveComponent.CreateDynamicMaterialInstance` (`self.StaticMesh`) 0 "/Game/StudentWork/Materials/M_ControlledFlash.M_ControlledFlash" "None"))
  (set `self.Flash Material` _returnvalue))