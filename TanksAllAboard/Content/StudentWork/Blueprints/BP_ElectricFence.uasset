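; BP_ElectricFence is a fence hazard that hurts the player on entering its collision box while electrified.
; On overlap it casts to BP_PlayerCharacter, applies damage and sends a negative score message to the player controller.
; Each hit briefly swaps the fence materials, restoring M_Grate two ticks later.
; The looping damage timer setup is disconnected, so damage lands once per entry, although end overlap still clears the timer.
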(event `self.BoxCollision.OnComponentEndOverlap`
  (params (OverlappedComponent :type "PrimitiveComponent Object Reference") (OtherActor :type "Actor Object Reference") (OtherComp :type "PrimitiveComponent Object Reference") (OtherBodyIndex :type Integer))
  ;[1 1 1] Clear Timer
  (`KismetSystemLibrary.K2_ClearAndInvalidateTimerHandle` (`self.ElectricTimer`)))

(event `ElectricDamage`
  ;[1 0.03953 0.04947] Damage
  (if (`self.IsElectrified`) :!label _label
    (`GameplayStatics.ApplyDamage` (stale `self.BoxCollision.OnComponentBeginOverlap` _asbp_player_character) 10.0)
    (message `/Game/BI_score.I_UpdateScore` (`GameplayStatics.GetPlayerController` 0) -10.0)
    ;[0.3567 0.9342 1] Material Changes
    (`PrimitiveComponent.SetMaterial` (`self.Fence`) 0 "/Game/Materials/MI_Grate1.MI_Grate1")
    (`PrimitiveComponent.SetMaterial` (`self.Fence`) 0 "/Game/Materials/MI_Grate1.MI_Grate1")
    (`PrimitiveComponent.SetMaterial` (`self.Plane`) 0 "/Game/Materials/MI_Grate1.MI_Grate1")
    (`KismetSystemLibrary.DelayUntilNextTick`)
    (`KismetSystemLibrary.DelayUntilNextTick`)
    (`PrimitiveComponent.SetMaterial` (`self.Fence`) 0 "/Game/Materials/M_Grate.M_Grate")
    (`PrimitiveComponent.SetMaterial` (`self.Fence`) 0 "/Game/Materials/M_Grate.M_Grate")
    (`PrimitiveComponent.SetMaterial` (`self.Plane`) 0 "/Game/Materials/M_Grate.M_Grate")))

(event `self.BoxCollision.OnComponentBeginOverlap`
  (params (OverlappedComponent :type "PrimitiveComponent Object Reference") (OtherActor :type "Actor Object Reference") (OtherComp :type "PrimitiveComponent Object Reference") (OtherBodyIndex :type Integer) (bFromSweep :type Boolean) (SweepResult :type "HitResult Structure (by ref)"))
  (bind _asbp_player_character (cast `/Game/Blueprints/BP_PlayerCharacter` OtherActor))
  (goto _label))

(fn `UserConstructionScript`)