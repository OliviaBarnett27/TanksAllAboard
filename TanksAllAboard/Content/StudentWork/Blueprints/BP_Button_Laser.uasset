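; BP_Button_Laser is a damageable button that switches off its linked laser gate when destroyed.
; The first damage event plays a flash timeline driving the FlashLevel parameter on a dynamic material created in the construction script.
; When the flash finishes, it spawns burst and crumble effects, sends a score update to the player controller through an interface, destroys itself and calls DisableLasers on MyLaserGate.
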(event `self.ReceiveAnyDamage`
  (params (Damage :type "Float (single-precision)") (DamageType :type "DamageType Object Reference") (InstigatedBy :type "Controller Object Reference") (DamageCauser :type "Actor Object Reference"))
  (bind _returnvalue (`SceneComponent.K2_GetComponentLocation` (`self.Cube`)))
  (`/Engine/EditorBlueprintResources/StandardMacros.DoOnce` false
    (:`Completed`
      ;[1 0.4895 0.4994] Flashing Effect
      (bind (_direction _flash) (`Timeline|TL_Flash`)
        (:`Update`
          (`MeshComponent.SetScalarParameterValueOnMaterials` (`self.Cylinder`) "FlashLevel" _flash))
        (:`Finished`
          ;[0.6978 0.296 1] Systems
          (`NiagaraFunctionLibrary.SpawnSystemAtLocation` "/Game/StudentWork/Systems/NS_UpwardMeshBurst.NS_UpwardMeshBurst" _returnvalue)
          (set `self.Explosion` null)
          (`NiagaraFunctionLibrary.SpawnSystemAtLocation` "/Game/StudentWork/Systems/NS_Crumble2.NS_Crumble2" _returnvalue)
          (message `/Game/BI_score.I_UpdateScore` (`GameplayStatics.GetPlayerController` 0) 50.0)
          ;[1 0 0.3645] Disable Lasers (from BP_LaserGate)
          (`self.K2_DestroyActor`)
          (`/Game/StudentWork/Blueprints/BP_LaserGate.DisableLasers` (`self.MyLaserGate`)))))))

(fn `UserConstructionScript`
  (bind _returnvalue (`PrimitiveComponent.CreateDynamicMaterialInstance` (`self.Cylinder`) 0 "/Game/StudentWork/Materials/M_Flashing.M_Flashing" "None"))
  (set `self.FlashMaterial` _returnvalue))