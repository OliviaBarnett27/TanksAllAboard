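; BP_BasicTurret is a destructible enemy turret that fires projectiles automatically.
; A looping timer started on BeginPlay spawns BP_EnemyProjectile at the Arrow component's location and rotation.
; When IsRotate is set, a timeline lerps the static mesh between start and target rotations.
; Any damage removes a fixed amount of Health; at zero it destroys itself and sends score through an interface message to the player controller.
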(event `self.ReceiveAnyDamage`
  (params (Damage :type "Float (single-precision)") (DamageType :type "DamageType Object Reference") (InstigatedBy :type "Controller Object Reference") (DamageCauser :type "Actor Object Reference"))
  ;[1 0 0] Damage
  (set `self.Health` (- (`self.Health`) 30.0))
  (if (not (> (`self.Health`) 0.0))
    (`self.K2_DestroyActor`)
    (message `/Game/BI_score.I_UpdateScore` (`GameplayStatics.GetPlayerController` 0) 75.0)))

(event `self.ReceiveBeginPlay`
  ;[1 0.6038 0.1531] Firing
  (bind _returnvalue (`KismetSystemLibrary.K2_SetTimerDelegate` (delegate `Fire Projectile`) 0.5 true))
  (set `self.FireTimer` _returnvalue)
  (if (`self.Is Rotate?`)
    ;[0.6935 0.4267 1] Rotation
    (bind (_direction _alpha) (`Timeline|TL_Rotation`)
      (:`Update`
        (`SceneComponent.K2_SetRelativeRotation` (`self.StaticMesh`) (`KismetMathLibrary.RLerp` (`self.Start Rotation`) (`self.Target Rotation`) _alpha) false false)))))

(event `Fire Projectile`
  (bind _arrow (`self.Arrow`))
  ;[1 0.6038 0.1531] Firing
  (`|SpawnActorFromClass` "/Game/StudentWork/Blueprints/Projectiles/BP_EnemyProjectile.BP_EnemyProjectile_C" (`KismetMathLibrary.MakeTransform` (`SceneComponent.K2_GetComponentLocation` _arrow) (`SceneComponent.K2_GetComponentRotation` _arrow)) "Undefined" "MultiplyWithRoot" null null))

(fn `UserConstructionScript`)